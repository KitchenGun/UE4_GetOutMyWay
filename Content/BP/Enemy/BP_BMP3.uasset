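; BP_BMP3 is an enemy BMP-3 tracked vehicle Blueprint that carries wheel smoke and dust trail effects.
; Its SetWheelSmokeIntensity event activates all left and right wheel VFX components and the dust trail when intensity is above zero, and deactivates them otherwise.
; The intensity value works only as an on/off switch, and the construction script is empty.
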(event Custom|SetWheelSmokeIntensity
  (params (Intensity :type Float%20%28single-precision%29))
  (Components|Activation|SetActive (Variables|Default|GetWheelVFX_R2) (> Intensity 0.0) false))

(fn ConstructionScript)