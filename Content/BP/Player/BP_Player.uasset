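; BP_Player is the player Blueprint, handling movement and camera-boom input.
; MoveForward moves along the flattened control-yaw forward vector, while MoveRight adds scaled controller yaw, turning rather than strafing.
; VerticalLook and HorizontalLook both trigger one relative SpringArm rotation that changes only yaw.
; A pitch-clamp calculation is present but unused, and the construction script is empty.
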(fn ConstructionScript)

(event Input|AxisEvents|InputAxisMoveRight
  (params (AxisValue :type Float%20%28single-precision%29))
  ;[1 1 1] LowerMoveEvent
  (Pawn|Input|AddControllerYawInput (* AxisValue 0.1)))

(event Input|AxisEvents|InputAxisMoveForward
  (params (AxisValue :type Float%20%28single-precision%29))
  ;[1 1 1] LowerMoveEvent
  (Pawn|Input|AddMovementInput (Class|KismetMathLibrary|VectorNormal2D (Math|Vector|GetForwardVector (Math|Rotator|MakeRotator 0.0 0.0 (.Yaw (Math|Rotator|BreakRotator (Pawn|GetControlRotation :!class /Script/Engine.Pawn))))) 0.0001) AxisValue false))

(event Input|AxisEvents|InputAxisHorizontalLook
  (params (AxisValue :type Float%20%28single-precision%29))
  (Transformation|AddRelativeRotation (Variables|Default|GetSpringArm) (Math|Rotator|MakeRotator 0.0 0.0 AxisValue) false false))

(event Input|AxisEvents|InputAxisVerticalLook
  (params (AxisValue :type Float%20%28single-precision%29))
  (Transformation|AddRelativeRotation (Variables|Default|GetSpringArm) (Math|Rotator|MakeRotator 0.0 0.0 (stale Input|AxisEvents|InputAxisHorizontalLook AxisValue)) false false))