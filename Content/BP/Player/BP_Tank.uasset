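; BP_Tank is a player-controlled tank pawn that drives and turns from axis inputs and aims with control rotation.
; It caches the M1A1 Abrams AnimBP on BeginPlay and writes wheel speed to it from movement input.
; Tick steps the AnimBP's turret angle and gun elevation until near control yaw and pitch.
; Both only step by adding their speed, as the subtracting nodes are unconnected.
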(event EventTick
  (params (DeltaSeconds :type Float%20%28single-precision%29))
  (bind _tankabp (Variables|AnimationBP|GetTankABP))
  (bind _tankabp_2 (Variables|AnimationBP|GetTankABP))
  (Utilities|FlowControl|Sequence
    (:then_0
      (if (Math|Float|NearlyEqual(Float) (Variables|/Game/VigilanteContent/Vehicles/West_Tank_M1A1Abrams/ABP_West_Tank_M1A1Abrams.ABP_West_Tank_M1A1Abrams_C|GetTurretAngle (Variables|AnimationBP|GetTankABP)) (.yaw (Pawn|GetControlRotation :!class /Script/Engine.Pawn)) 3.0)
        (Development|PrintString "set")
        (elif true
          (if (not (> (+ (Variables|TankMovement|GetTurretTurnSpeed) (Variables|/Game/VigilanteContent/Vehicles/West_Tank_M1A1Abrams/ABP_West_Tank_M1A1Abrams.ABP_West_Tank_M1A1Abrams_C|GetTurretAngle _tankabp_2)) 3.6e+02))
            (Variables|/Game/VigilanteContent/Vehicles/West_Tank_M1A1Abrams/ABP_West_Tank_M1A1Abrams.ABP_West_Tank_M1A1Abrams_C|SetTurretAngle _tankabp_2 (+ (Variables|TankMovement|GetTurretTurnSpeed) (Variables|/Game/VigilanteContent/Vehicles/West_Tank_M1A1Abrams/ABP_West_Tank_M1A1Abrams.ABP_West_Tank_M1A1Abrams_C|GetTurretAngle _tankabp_2)))))))
    (:then_1
      (if (not (Math|Float|NearlyEqual(Float) (Variables|/Game/VigilanteContent/Vehicles/West_Tank_M1A1Abrams/ABP_West_Tank_M1A1Abrams.ABP_West_Tank_M1A1Abrams_C|GetGunElevation (Variables|AnimationBP|GetTankABP)) (.pitch (Pawn|GetControlRotation :!class /Script/Engine.Pawn)) 5.0))
        (Variables|/Game/VigilanteContent/Vehicles/West_Tank_M1A1Abrams/ABP_West_Tank_M1A1Abrams.ABP_West_Tank_M1A1Abrams_C|SetGunElevation _tankabp (+ (Variables|TankMovement|GetGunElevationSpeed) (Variables|/Game/VigilanteContent/Vehicles/West_Tank_M1A1Abrams/ABP_West_Tank_M1A1Abrams.ABP_West_Tank_M1A1Abrams_C|GetGunElevation _tankabp)))))))

(event Input|AxisEvents|InputAxisMoveForward
  (params (AxisValue :type Float%20%28single-precision%29))
  (bind _forwardzspeed (Variables|TankMovement|GetForwardZSpeed))
  (bind _returnvalue (* AxisValue _forwardzspeed))
  ;[1 1 1] MoveForward
  (Transformation|AddActorLocalOffset (Math|Vector|MakeVector _returnvalue 0.0 0.0) false false)
  (Variables|/Game/VigilanteContent/Vehicles/West_Tank_M1A1Abrams/ABP_West_Tank_M1A1Abrams.ABP_West_Tank_M1A1Abrams_C|SetWheelSpeed (Variables|AnimationBP|GetTankABP) (* _returnvalue 1e+02)))

(event Input|AxisEvents|InputAxisMoveRight
  (params (AxisValue :type Float%20%28single-precision%29))
  (bind _turnspeed (Variables|TankMovement|GetTurnSpeed))
  (bind _returnvalue (* AxisValue _turnspeed))
  ;[1 1 1] MoveRight
  (Transformation|AddActorLocalRotation (Math|Rotator|MakeRotator 0.0 0.0 _returnvalue) false false)
  (Variables|/Game/VigilanteContent/Vehicles/West_Tank_M1A1Abrams/ABP_West_Tank_M1A1Abrams.ABP_West_Tank_M1A1Abrams_C|SetWheelSpeed (Variables|AnimationBP|GetTankABP) (* _returnvalue 1e+02)))

(event Input|AxisEvents|InputAxisVerticalLook
  (params (AxisValue :type Float%20%28single-precision%29))
  (Pawn|Input|AddControllerPitchInput AxisValue))

(event Input|AxisEvents|InputAxisHorizontalLook
  (params (AxisValue :type Float%20%28single-precision%29))
  (bind _returnvalue (Pawn|GetControlRotation :!class /Script/Engine.Pawn))
  (Pawn|Input|AddControllerYawInput AxisValue)
  (Pawn|SetControlRotation (Game|GetPlayerController 0) (Math|Rotator|MakeRotator 0.0 (.pitch _returnvalue) (.yaw _returnvalue))))

(fn ConstructionScript)

(event EventBeginPlay
  (bind _asabp_west_tank_m1a1abrams (Utilities|Casting|CastToABP_West_Tank_M1A1Abrams (Components|SkeletalMesh|GetAnimInstance (Variables|Default|GetSkeletalMesh self))))
  (bind _output_get (Variables|AnimationBP|SetTankABP _asabp_west_tank_m1a1abrams))
  (Variables|/Game/VigilanteContent/Vehicles/West_Tank_M1A1Abrams/ABP_West_Tank_M1A1Abrams.ABP_West_Tank_M1A1Abrams_C|SetHatchAngle _output_get 0.0))